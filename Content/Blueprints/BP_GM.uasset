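; Game manager for a circuit puzzle that starts current flow through BP_Board pieces and detects the win.
; BeginPlay gathers the pieces and builds a lamp list, which events can edit.
; CircuitFlow triggers type-2 pieces and starts a one-second countdown that checks lamps, where the last lamp's state decides victory.
; Victory fires once and pauses the timer, while an expired countdown de-electrifies all pieces and re-arms the win check.
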(event `CircuitFlow`
  (for _array_element (`self.AllPieces`)
    (if (== (`/Game/Blueprints/BP_Board.PieceType` _array_element) 2)
      (`/Game/Blueprints/BP_Board.FlowProceed` _array_element)
      (bind _returnvalue (`KismetSystemLibrary.K2_SetTimerDelegate` (delegate `Countdown`) 1.0 true))
      ;[0.3008 0.7127 1] Comment
      (set `self.CircuitTimer` _returnvalue))))

(event `Countdown`
  (bind _circuitcooldown (`self.CircuitCooldown`))
  (if (> _circuitcooldown 0.0)
    (bind _result (`/Engine/EditorBlueprintResources/StandardMacros.DecrementFloat` _circuitcooldown)
      (:`  `
        (set `self.CircuitCooldown` _result)
        ;[0.1137 0.6521 1] Comment
        (for _array_element (`self.LampList`)
          (if (`/Game/Blueprints/BP_Board.IsElectrified` _array_element)
            (set `self.isWinnable` true)
            (else
              (set `self.isWinnable` false))))
        (if (`self.isWinnable`)
          (`/Engine/EditorBlueprintResources/StandardMacros.DoOnce` false :!label _label
            (:`Completed`
              (`KismetSystemLibrary.PrintString` "Win")
              (`self.Victory`))))))
    (else
      (for _array_element_2 (`self.AllPieces`)
        (set `/Game/Blueprints/BP_Board.IsElectrified` false _array_element_2)
        (`PrimitiveComponent.SetMaterialByName` (`/Game/Blueprints/BP_Board.Cube` _array_element_2) "WireSlot" "/Game/Materials/bulb_light_004.bulb_light_004")
        (set `self.FlowPitchCombo` 0.0))
      (goto _label :!via `Reset`))))

(event `self.ReceiveBeginPlay`
  ;[0.2027 0.6159 1] Comment
  (add `self.Victory` (delegate `Victory_Event`))
  (bind _outactors (`GameplayStatics.GetAllActorsOfClass` "/Game/Blueprints/BP_Board.BP_Board_C"))
  (bind _output_get (set `self.AllPieces` _outactors))
  (for _array_element _output_get
    (switch `/Game/DataOrganization/ENUM_PieceTypes` (`/Game/Blueprints/BP_Board.PieceType` _array_element)
      (:`NewEnumerator3`
        (`KismetArrayLibrary.Array_AddUnique` (`self.LampList`) _array_element)))))

(event `Victory_Event`
  ;[0.2027 0.6159 1] Comment
  (set `self.isWon` true)
  (`KismetSystemLibrary.K2_PauseTimerHandle` (`self.CircuitTimer`)))

(event `AddLampToLampList`
  (params (Lamp :type "/Game/Blueprints/BP_Board Object Reference"))
  ;[0.2027 0.6159 1] Comment
  (`KismetArrayLibrary.Array_AddUnique` (`self.LampList`) Lamp))

(event `RemoveLampFromLampList`
  (params (Lamp :type "/Game/Blueprints/BP_Board Object Reference"))
  (bind _lamplist (`self.LampList`))
  ;[0.2027 0.6159 1] Comment
  (if (`KismetArrayLibrary.Array_Contains` _lamplist Lamp)
    (`KismetArrayLibrary.Array_RemoveItem` _lamplist Lamp)))

(fn `UserConstructionScript`)