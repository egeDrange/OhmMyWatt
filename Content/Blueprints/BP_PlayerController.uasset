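; BP_PlayerController sets up mouse-driven play, viewed through a placed camera, for what its input mapping suggests is a board-piece game.
; On BeginPlay it shows the cursor, uses Game and UI input, and blends the view to the first BP_Camera found.
; It then adds the WBP_ComponentMenu widget to the viewport and registers the IM_BoardPiece Enhanced Input mapping context.
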(event `self.ReceiveBeginPlay`
  (set `self.bShowMouseCursor` true)
  (`WidgetBlueprintLibrary.SetInputMode_GameAndUIEx` self null "DoNotLock" false)
  (bind _outactors (`GameplayStatics.GetAllActorsOfClass` "/Game/Blueprints/BP_Camera.BP_Camera_C"))
  (`self.SetViewTargetWithBlend` (`PlayerState.GetPlayerController` (`GameplayStatics.GetPlayerState` 0)) (`|GetArrayItem` _outactors) 0.0 "VTBlend_Linear" 0.0 false)
  (bind _returnvalue (`|GenericCreateObject` "/Game/Blueprints/WBP_ComponentMenu.WBP_ComponentMenu_C"))
  (`UserWidget.AddToViewport` _returnvalue 0)
  (`EnhancedInputSubsystemInterface.AddMappingContext` (pcsubsystem `EnhancedInputLocalPlayerSubsystem` (`GameplayStatics.GetPlayerController` 0)) "/Game/Input/IM_BoardPiece.IM_BoardPiece" 0 (struct)))

(fn `UserConstructionScript`)