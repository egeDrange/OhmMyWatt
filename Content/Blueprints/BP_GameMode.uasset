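; Game mode for a circuit puzzle that starts current flow, resets the board and handles level progression.
; CircuitFlow triggers FlowProceed on type-4 pieces and starts a looping countdown that, once expired, de-electrifies all pieces and plays a one-shot reset sound.
; BeginPlay increments the game instance's level and gathers pieces and lamps; Victory stops the timer and opens the next numbered map after a delay.
; The old all-lamps win check is disconnected.
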(event `CircuitFlow`
  (for _array_element (`self.AllPieces`)
    (if (== (`/Game/Blueprints/BP_Boardpiece.PieceType` _array_element) 4)
      (`/Game/Blueprints/BP_Boardpiece.FlowProceed` _array_element)
      ;[0.5841 0.2705 1] VictoryCondition (Old)
      (bind _returnvalue (`KismetSystemLibrary.K2_SetTimerDelegate` (delegate `Countdown`) 1.0 true))
      (set `self.CircuitTimer` _returnvalue)
      (goto _label :!via `Reset`))))

(event `Countdown`
  (if (> (`self.CircuitCooldown`) 0.0)
    (bind _result (`/Engine/EditorBlueprintResources/StandardMacros.DecrementFloat` (`self.CircuitCooldown`))
      (:`  `
        (set `self.CircuitCooldown` _result)))
    (else
      (for _array_element (`self.AllPieces`)
        (set `/Game/Blueprints/BP_Boardpiece.IsElectrified` false _array_element)
        (`PrimitiveComponent.SetMaterialByName` (`/Game/Blueprints/BP_Boardpiece.Cube` _array_element) "WireSlot" "/Game/Materials/bulb_light_004.bulb_light_004")
        (set `self.FlowPitchCombo` 0.0)
        (`/Engine/EditorBlueprintResources/StandardMacros.DoOnce` false :!label _label
          (:`Completed`
            (`GameplayStatics.PlaySoundAtLocation` (`self.CircuitResetSound`) (0.0 0.0 0.0) (struct) 1.0 1.0 0.0 null null null null))))
      ;[0.5841 0.2705 1] VictoryCondition (Old)
      (`/Engine/EditorBlueprintResources/StandardMacros.DoOnce` false :!via `Reset`
        (:`Completed`
          (`KismetSystemLibrary.PrintString` "Won")
          (`self.Victory`))))))

(event `self.ReceiveBeginPlay`
  ;[0.2086 0.5711 1] LampList
  (bind _asbp_game_instance (cast `/Game/Blueprints/BP_GameInstance` (`GameplayStatics.GetGameInstance`)))
  (`/Engine/EditorBlueprintResources/StandardMacros.IncrementInt` (`/Game/Blueprints/BP_GameInstance.Level` _asbp_game_instance)
    (:`  `
      (add `self.Victory` (delegate `Victory_Event`))
      (bind _outactors (`GameplayStatics.GetAllActorsOfClass` "/Game/Blueprints/BP_Boardpiece.BP_Boardpiece_C"))
      (bind _output_get (set `self.AllPieces` _outactors))
      (for _array_element _output_get
        (switch `/Game/DataOrganization/ENUM_PieceTypes` (`/Game/Blueprints/BP_Boardpiece.PieceType` _array_element)
          (:`NewEnumerator3`
            (`KismetArrayLibrary.Array_AddUnique` (`self.LampList`) _array_element)))))))

(event `Victory_Event`
  ;[0.2086 0.5711 1] LampList
  (set `self.isWon` true)
  (`KismetSystemLibrary.K2_PauseTimerHandle` (`self.CircuitTimer`))
  (`KismetSystemLibrary.Delay` 5.0)
  (`GameplayStatics.OpenLevel` (`KismetStringLibrary.Conv_StringToName` (`KismetStringLibrary.Concat_StrStr` "M_Level" (`KismetStringLibrary.Conv_IntToString` (+ (`/Game/Blueprints/BP_GameInstance.Level` (stale `self.ReceiveBeginPlay` _asbp_game_instance)) 1))))))

(event `AddLampToLampList`
  (params (Lamp :type "/Game/Blueprints/BP_Boardpiece Object Reference"))
  ;[0.2086 0.5711 1] LampList
  ;;[0.9204 0.3093 1] Victory Condition (Old)
  (`KismetArrayLibrary.Array_AddUnique` (`self.LampList`) Lamp))

(event `RemoveLampFromLampList`
  (params (Lamp :type "/Game/Blueprints/BP_Boardpiece Object Reference"))
  (bind _lamplist (`self.LampList`))
  ;[0.2086 0.5711 1] LampList
  ;;[0.9204 0.3093 1] Victory Condition (Old)
  (if (`KismetArrayLibrary.Array_Contains` _lamplist Lamp)
    (`KismetArrayLibrary.Array_RemoveItem` _lamplist Lamp)))

(fn `UserConstructionScript`)