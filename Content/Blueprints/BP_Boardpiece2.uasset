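; Board tile for a circuit-building puzzle, holding one component such as a cell, lamp, cable or resistor.
; Initially Missing tiles highlight on hover, take the GameMode's selected type on click, and rotate with an animated lift.
; A DataTable sets each type's mesh, while type-specific side colliders let FlowProceed recursively electrify overlapping neighbours with rising pitch.
; Lamps register with the GameMode, whose Victory event locks tiles and raises buildings.
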(event `Victory_Event`
  ;[0.1893 0.6277 1] Comment
  (set `self.IsInteractable` false)
  (`self.WinAnimation`))

(event `self.ReceiveBeginPlay`
  (`self.UpdatePiece`)
  (bind _asbp_game_mode (cast `/Game/Blueprints/BP_GameMode2` (`GameplayStatics.GetGameMode`)))
  (set `self.GameModeRef` _asbp_game_mode)
  (`self.InteractableCheck`)
  (add `self.OnBeginCursorOver` (delegate `OnHovered`))
  (add `self.OnEndCursorOver` (delegate `OnExitHover`))
  (add `self.OnClicked` (delegate `OnClicked_Event`))
  ;[0.5776 1 0.2664] For Rotation Mechanic
  (`self.EnableInput` (`GameplayStatics.GetPlayerController` 0))
  (set `self.CurrentRotation` (`self.K2_GetActorRotation`))
  (set `self.StartLocation` (`self.K2_GetActorLocation`))
  ;[0.1893 0.6277 1] Comment
  (add `/Game/Blueprints/BP_GameMode2.Victory` (`self.GameModeRef`) (delegate `Victory_Event`)))

(event `OnHovered` :!signature `self.OnBeginCursorOver`
  (params (TouchedActor :type "Actor Object Reference"))
  (if (`self.IsInteractable`)
    (`MeshComponent.SetOverlayMaterial` (`self.Cube`) "/Game/Materials/M_HighlightOverlay.M_HighlightOverlay")
    (set `self.IsHovered` true)))

(event `OnExitHover` :!signature `self.OnEndCursorOver`
  (params (TouchedActor :type "Actor Object Reference"))
  (`MeshComponent.SetOverlayMaterial` (`self.Cube`) null)
  (set `self.IsHovered` false))

(event `OnClicked_Event` :!signature `self.OnClicked`
  (params (TouchedActor :type "Actor Object Reference") (ButtonPressed :type "Key Structure" :default "None"))
  (if (`self.IsInteractable`)
    (switch `string` (`/Game/Blueprints/BP_GameMode2.SelectedPieceType` (`self.GameModeRef`))
      (:`Missing`
        (set `self.PieceType` "NewEnumerator0")
        ;[0.1721 0.7047 1] Comment
        (`self.RemoveFromLampList`))
      (:`Cell`
        (set `self.PieceType` "NewEnumerator2")
        (`self.RemoveFromLampList`))
      (:`Lamp`
        (set `self.PieceType` "NewEnumerator3")
        (`self.AddToLampList`))
      (:`Cable`
        (set `self.PieceType` "NewEnumerator1")
        (`self.RemoveFromLampList`))
      (:`Resistor`
        (set `self.PieceType` "NewEnumerator4")
        (`self.RemoveFromLampList`))
      (:`Ampermeter`
        (set `self.PieceType` "NewEnumerator5")
        (`self.RemoveFromLampList`))
      (:`Voltmeter`
        (set `self.PieceType` "NewEnumerator6")
        (`self.RemoveFromLampList`)))
    (`self.UpdatePiece`)))

(event `FlowProceed`
  (bind _gamemoderef (`self.GameModeRef`))
  (`GameplayStatics.PlaySoundAtLocation` (`self.FlowProceedSFX`) (0.0 0.0 0.0) (struct) 1.0 (`/Game/Blueprints/BP_GameMode2.FlowPitchCombo` (`self.GameModeRef`)) 0.0 null null null null)
  ;[0.2488 0.5782 1] Comment
  (if (not (`self.IsElectrified`))
    (set `/Game/Blueprints/BP_GameMode2.CircuitCooldown` 3.0 (`self.GameModeRef`))
    (set `self.IsElectrified` true)
    (`PrimitiveComponent.SetMaterialByName` (`self.Cube`) "WireSlot" "/Game/Materials/bulb_black.bulb_black")
    (for _array_element (`self.CollidersArray`)
      (for _array_element_2 (`PrimitiveComponent.GetOverlappingComponents` _array_element)
        (bind _asbp_boardpiece (cast `/Game/Blueprints/BP_Boardpiece2` (`ActorComponent.GetOwner` _array_element_2)))
        (if (not (`/Game/Blueprints/BP_Boardpiece2.IsElectrified` _asbp_boardpiece))
          (set `/Game/Blueprints/BP_GameMode2.FlowPitchCombo` (+ (`/Game/Blueprints/BP_GameMode2.FlowPitchCombo` _gamemoderef) 0.25) _gamemoderef)
          (`self.FlowProceed` _asbp_boardpiece))))))

(event `EnhancedInput|/Game/Input/IA_Rotate`
  (params (ActionValue :type Boolean) (ElapsedSeconds :type "Float (double-precision)") (TriggeredSeconds :type "Float (double-precision)") (InputAction :type "InputAction Object Reference" :default "/Game/Input/IA_Rotate.IA_Rotate"))
  (bind _startlocation (`self.StartLocation`))
  (bind (_currentrotation_roll _currentrotation_pitch _currentrotation_yaw) (`KismetMathLibrary.BreakRotator` (`self.CurrentRotation`)))
  ;[0.5776 1 0.2664] Rotation Logic
  (:`Triggered`
    (if (and (`self.IsHovered`) (`self.IsInteractable`))
      (set `self.IsInteractable` false)
      (bind (_direction _liftcurve _rotatecurve) (`Timeline|RotateTimeline` :!via `PlayFromStart`)
        (:`Update`
          (`|ExecutionSequence`
            (:`then_0`
              (`self.K2_SetActorLocation` (`KismetMathLibrary.VLerp` _startlocation (+ _startlocation (0.0 0.0 10.0)) _liftcurve)))
            (:`then_1`
              (`self.K2_SetActorRotation` (`KismetMathLibrary.RLerp` (`self.CurrentRotation`) (`KismetMathLibrary.MakeRotator` _currentrotation_roll _currentrotation_pitch (+ _currentrotation_yaw 90.0)) _rotatecurve)))))
        (:`Finished`
          (set `self.CurrentRotation` (`self.K2_GetActorRotation`))
          (set `self.IsInteractable` true))))))

(event `WinAnimation`
  (bind _buildings (`self.Buildings`))
  (bind _returnvalue (`SceneComponent.K2_GetComponentLocation` _buildings))
  ;[1 1 1] Comment
  (`KismetSystemLibrary.PrintString` "Playing win anim")
  (`SceneComponent.SetVisibility` (`self.Buildings`) true false)
  (bind (_direction _height_of_buildings) (`Timeline|Timeline_0` :!via `PlayFromStart`)
    (:`Update`
      (`SceneComponent.K2_SetWorldLocation` _buildings (`KismetMathLibrary.VLerp` _returnvalue (+ _returnvalue (0.0 0.0 0.2)) _height_of_buildings) false false))))

(fn `AddToLampList`
  (`/Game/Blueprints/BP_GameMode2.AddLampToLampList` (`self.GameModeRef`) self))

(fn `InteractableCheck`
  (if (`KismetStringLibrary.EqualEqual_StrStr` (`|GetEnumeratorNameAsString` (`self.PieceType`)) "Missing")
    (set `self.IsInteractable` true)))

(fn `RemoveFromLampList`
  (`/Game/Blueprints/BP_GameMode2.RemoveLampFromLampList` (`self.GameModeRef`) self))

(fn `UpdatePiece`
  (bind _returnvalue (`|GetDataTableRow` (`self.DataTable`) (`KismetStringLibrary.Conv_StringToName` (`|GetEnumeratorNameAsString` (`self.PieceType`))))
    (:`then`
      (bind (_piecetype _piecemesh) (break `/Game/DataOrganization/STR_PieceToColor` _returnvalue))
      (`StaticMeshComponent.SetStaticMesh` (`self.Cube`) _piecemesh)
      (for _array_element (`self.CollidersArray`)
        (`PrimitiveComponent.SetCollisionEnabled` _array_element "NoCollision"))
      (switch `/Game/DataOrganization/ENUM_PieceTypes` _piecetype
        (:`NewEnumerator1`
          (`PrimitiveComponent.SetCollisionEnabled` (`|GetArrayItem` (`self.CollidersArray`)) "QueryAndProbe" :!label _label)
          (`PrimitiveComponent.SetCollisionEnabled` (`|GetArrayItem` (`self.CollidersArray`) 1) "QueryAndProbe"))
        (:`NewEnumerator2`
          (`PrimitiveComponent.SetCollisionEnabled` (`self.SouthC`) "QueryAndProbe")
          (`PrimitiveComponent.SetCollisionEnabled` (`|GetArrayItem` (`self.CollidersArray`) 1) "QueryAndProbe"))
        (:`NewEnumerator3`
          (`PrimitiveComponent.SetCollisionEnabled` (`|GetArrayItem` (`self.CollidersArray`) 2) "QueryAndProbe")
          (`PrimitiveComponent.SetCollisionEnabled` (`|GetArrayItem` (`self.CollidersArray`) 3) "QueryAndProbe"))
        (:`NewEnumerator4`
          (goto _label))))))

(fn `UserConstructionScript`
  (`SceneComponent.SetVisibility` (`self.PlainTerrain`) false false)
  (`SceneComponent.SetVisibility` (`self.Buildings`) false false)
  (set `self.CollidersArray` (`|MakeArray` (`self.NorthC`) (`self.SouthC`) (`self.EastC`) (`self.WestC`)))
  (`self.UpdatePiece`))